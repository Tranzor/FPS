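; Repair pickup that restores the player's HOLLO vehicle, cached along with its mesh on BeginPlay.
; Any actor overlap triggers it if the vehicle's DamageLevel is at or above a threshold; the overlapping actor is not checked.
; It clears damage and damage-stage flags and zeroes the directional dent morph targets on the mesh.
; It hides its mesh and disables sphere collision, then reappears after a short delay.
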(event `self.ReceiveBeginPlay`
  (bind _ashollo (cast `/Game/CarTest/Blueprints/HOLLO/HOLLO` (`GameplayStatics.GetPlayerPawn` 0)))
  (bind _output_get (set `self.VehicleReference` _ashollo))
  (set `self.VehicleMeshReference` (`WheeledVehicle.Mesh` _output_get)))

(event `self.ReceiveActorBeginOverlap`
  (params (OtherActor :type "Actor Object Reference"))
  (if (>= (`/Game/CarTest/Blueprints/HOLLO/HOLLO.DamageLevel` (`self.VehicleReference`)) 5.0)
    (set `/Game/CarTest/Blueprints/HOLLO/HOLLO.DamageLevel` 0.0 (`self.VehicleReference`))
    (`SceneComponent.SetVisibility` (`self.StaticMeshComponent`) false false)
    (`PrimitiveComponent.SetCollisionEnabled` (`self.Sphere`) "NoCollision")
    (`|ExecutionSequence`
      (:`then_0`
        (`SkeletalMeshComponent.SetMorphTarget` (`self.VehicleMeshReference`) "Front" 0.0 true))
      (:`then_1`
        (`SkeletalMeshComponent.SetMorphTarget` (`self.VehicleMeshReference`) "Back" 0.0 true))
      (:`then_2`
        (`SkeletalMeshComponent.SetMorphTarget` (`self.VehicleMeshReference`) "Left" 0.0 true))
      (:`then_3`
        (`SkeletalMeshComponent.SetMorphTarget` (`self.VehicleMeshReference`) "Right" 0.0 true))
      (:`then_4`
        (`SkeletalMeshComponent.SetMorphTarget` (`self.VehicleMeshReference`) "Top" 0.0 true))
      (:`then_5`
        (`SkeletalMeshComponent.SetMorphTarget` (`self.VehicleMeshReference`) "FrontRCorner" 0.0 true))
      (:`then_6`
        (`SkeletalMeshComponent.SetMorphTarget` (`self.VehicleMeshReference`) "FrontLCorner" 0.0 true))
      (:`then_7`
        (`SkeletalMeshComponent.SetMorphTarget` (`self.VehicleMeshReference`) "BackRCorner" 0.0 true))
      (:`then_8`
        (`SkeletalMeshComponent.SetMorphTarget` (`self.VehicleMeshReference`) "BackLCorner" 0.0 true))
      (:`then_9`
        (set `/Game/CarTest/Blueprints/HOLLO/HOLLO.IsDLevel1` false (`self.VehicleReference`))
        (set `/Game/CarTest/Blueprints/HOLLO/HOLLO.IsDLevel2` false (`self.VehicleReference`))
        (set `/Game/CarTest/Blueprints/HOLLO/HOLLO.IsDLevel3` false (`self.VehicleReference`)))
      (:`then_10`
        (`KismetSystemLibrary.Delay` 5.0)
        (`SceneComponent.SetVisibility` (`self.StaticMeshComponent`) true false)
        (`PrimitiveComponent.SetCollisionEnabled` (`self.Sphere`) "QueryOnly")))))

(fn `UserConstructionScript`)