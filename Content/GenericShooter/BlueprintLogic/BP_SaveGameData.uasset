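; BP_SaveGameData holds the player's saved cosmetic choices: character, hat and hat color IDs.
; SetSavedVisuals compares each incoming ID with the stored one and overwrites only those that differ.
; Any change sets a SomethingChanged flag, which the function returns to its caller.
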(fn SetSavedVisuals
  (params (NewCharacterID :type Integer) (NewHatID :type Integer) (NewHatColorID :type Integer))
  (Utilities|FlowControl|Sequence
    (:then_0
      (if (!= NewCharacterID (Variables|Default|GetCharacterID))
        (Variables|Default|SetCharacterID NewCharacterID)
        (LocalVariables|SetbSomethingChanged true)))
    (:then_1
      (if (!= NewHatID (Variables|Default|GetHatID))
        (Variables|Default|SetHatID NewHatID)
        (LocalVariables|SetbSomethingChanged true)))
    (:then_2
      (if (!= NewHatColorID (Variables|Default|GetHatColorID))
        (Variables|Default|SetHatColorID NewHatColorID)
        (LocalVariables|SetbSomethingChanged true)))
    (:then_3
      (return (LocalVariables|GetbSomethingChanged)))))