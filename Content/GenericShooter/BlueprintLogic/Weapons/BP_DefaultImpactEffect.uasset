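; Weapon impact effect actor that plays surface-specific particles, sound and a decal where a shot hits.
; On BeginPlay, the physical material in HitInfo picks each asset through per-surface lookup functions, using Default when none exists.
; Decals attach to the hit component and bone with random roll, and the actor is flagged to auto-destroy when finished.
; Grass reuses the Glass particle effect, though its sound and decal are separate.
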(event EventBeginPlay
  (bind _hitinfo (Variables|Default|GetHitInfo))
  (bind (_bblockinghit _binitialoverlap _time _location _impactpoint _normal _impactnormal _physmat _hitactor _hitcomponent _hitbonename) (Collision|BreakHitResult _hitinfo))
  (bind _returnvalue (Utilities|IsValid _physmat))
  (bind _outrot (Utilities|VectortoRotator _impactnormal))
  (bind _surfacetype (Variables|/Script/Engine.PhysicalMaterial|GetSurfaceType _physmat))
  (bind (_roll _pitch _yaw) (Math|Rotator|BreakRotator _outrot))
  (bind _returnvalue_2 (select _returnvalue _surfacetype "SurfaceType_Default"))
  (bind _effect (CallFunction|GetEffect _returnvalue_2))
  (bind _soundcue (CallFunction|GetSound _returnvalue_2))
  (bind _decaldata (CallFunction|GetDecal _returnvalue_2))
  (bind (_material _size _lifespan) (Utilities|Struct|BreakSDecalData _decaldata))
  (Utilities|FlowControl|Sequence
    (:then_0
      ;[1 1 1] Spawn Particle Effect
      (Utilities|IsValid _effect
        (:Is%20Valid
          (Effects|SpawnEmitteratLocation _effect (Transformation|GetActorLocation) (Utilities|VectortoRotator _normal)))))
    (:then_1
      ;[1 1 1] Spawn Sound
      (Utilities|IsValid _soundcue
        (:Is%20Valid
          (Audio|PlaySoundatLocation _soundcue (Transformation|GetActorLocation)))))
    (:then_2
      ;[1 1 1] Spawn Decal
      (Utilities|IsValid _material
        (:Is%20Valid
          (Class|GameplayStatics|SpawnDecalAttached _material (Math|Vector|MakeVector _size _size 1.0) _hitcomponent _hitbonename _impactpoint (Math|Rotator|MakeRotator (Math|Random|RandomFloatinRange -1.8e+02 1.8e+02) _pitch _yaw) "KeepWorldPosition" _lifespan))))))

(fn ConstructionScript
  (Variables|Default|SetbAutoDestroyWhenFinished true))

(fn GetEffect
  (params (Surface :type EPhysicalSurface%20Enum :default "SurfaceType_Default"))
  (return (Utilities|Select :Index Surface :SurfaceType_Default (Variables|Defaults|GetDefaultEffect) :SurfaceType1 (Variables|Concrete|GetConcreteEffect) :SurfaceType2 (Variables|Dirt|GetDirtEffect) :SurfaceType3 (Variables|Water|GetWaterEffect) :SurfaceType4 (Variables|Metal|GetMetalEffect) :SurfaceType5 (Variables|Wood|GetWoodEffect) :SurfaceType6 (Variables|Glass|GetGlassEffect) :SurfaceType7 (Variables|Glass|GetGlassEffect) :SurfaceType8 (Variables|Flesh|GetFleshEffect))))

(fn GetSound
  (params (Surface :type EPhysicalSurface%20Enum :default "SurfaceType_Default"))
  (return (Utilities|Select :Index Surface :SurfaceType_Default (Variables|Defaults|GetDefaultSound) :SurfaceType1 (Variables|Concrete|GetConcreteSound) :SurfaceType2 (Variables|Dirt|GetDirtSound) :SurfaceType3 (Variables|Water|GetWaterSound) :SurfaceType4 (Variables|Metal|GetMetalSound) :SurfaceType5 (Variables|Wood|GetWoodSound) :SurfaceType6 (Variables|Grass|GetGrassSound) :SurfaceType7 (Variables|Glass|GetGlassSound) :SurfaceType8 (Variables|Flesh|GetFleshSound))))

(fn GetDecal
  (params (Surface :type EPhysicalSurface%20Enum :default "SurfaceType_Default"))
  (return (Utilities|Select :Index Surface :SurfaceType_Default (Variables|Defaults|GetDefaultDecal) :SurfaceType1 (Variables|Concrete|GetConcreteDecal) :SurfaceType2 (Variables|Dirt|GetDirtDecal) :SurfaceType3 (Variables|Water|GetWaterDecal) :SurfaceType4 (Variables|Metal|GetMetalDecal) :SurfaceType5 (Variables|Wood|GetWoodDecal) :SurfaceType6 (Variables|Grass|GetGrassDecal) :SurfaceType7 (Variables|Glass|GetGlassDecal) :SurfaceType8 (Variables|Flesh|GetFleshDecal))))